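; Interactable vault-door escape terminal that starts the escape defense when the player uses it with the escape console key.
; With the key, Interact consumes it, switches on every BP_AlarmLight and calls EscapeDefenseStart on BP_GameMode.
; Without the key, Interact toggles an info widget, which Tick removes once the player is over 200 units away.
; Tick also syncs the terminal's custom-depth highlight to key possession.
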(event EventBeginPlay
  (Variables|Default|SetWidgetClass "/Game/AlienHordeAssets/UI/Info/W_EscapeTerminalInfo.W_EscapeTerminalInfo_C"))

(event Collision|EventActorBeginOverlap
  (params (OtherActor :type Actor%20Object%20Reference)))

(event EventTick
  (params (DeltaSeconds :type Float%20%28single-precision%29))
  (bind _widget (Variables|Default|GetWidget))
  (bind _asbp_player_character (Utilities|Casting|CastToBP_PlayerCharacter (Game|GetPlayerCharacter 0)))
  (Rendering|SetRenderCustomDepth (Variables|Default|GetSM_Terminal_A) (Variables|/Game/AlienHordeAssets/Player/Blueprints/BP_PlayerCharacter.BP_PlayerCharacter_C|GetHasEscapeConsoleKey _asbp_player_character))
  (if (> (Math|Vector|Distance(Vector) (Transformation|GetWorldLocation (Variables|Default|GetStaticMesh)) (Transformation|GetActorLocation (Game|GetPlayerCharacter 0))) 2e+02)
    (Utilities|IsValid _widget
      (:Is%20Valid
        (Widget|RemovefromParent _widget)
        (Variables|Default|SetInteracted false)))))

(fn ConstructionScript
  (|CallParentFunction))

(fn Interact
  (params (Player :type BP%20Player%20Character%20Object%20Reference))
  (if (Variables|/Game/AlienHordeAssets/Player/Blueprints/BP_PlayerCharacter.BP_PlayerCharacter_C|GetHasEscapeConsoleKey Player)
    (Rendering|SetRenderCustomDepth (Variables|Default|GetSM_Terminal_A) false)
    (bind _outactors (Actor|GetAllActorsOfClass "/Game/AlienHordeAssets/Props/BP_AlarmLight.BP_AlarmLight_C"))
    (for _array_element _outactors
      (Default|TurnonLight _array_element))
    (bind _asbp_game_mode (Utilities|Casting|CastToBP_GameMode (Game|GetGameMode)))
    (Default|EscapeDefenseStart _asbp_game_mode)
    (Variables|/Game/AlienHordeAssets/Player/Blueprints/BP_PlayerCharacter.BP_PlayerCharacter_C|SetHasEscapeConsoleKey Player false)
    (elif (Variables|Default|GetInteracted)
      (Widget|RemovefromParent (Variables|Default|GetWidget))
      (Variables|Default|SetInteracted false)
      (else
        (bind _returnvalue (UserInterface|CreateWidget (Variables|Default|GetWidgetClass)))
        (bind _output_get (Variables|Default|SetWidget _returnvalue))
        (UserInterface|Viewport|AddtoViewport _output_get 0)
        (Variables|Default|SetInteracted true)))))