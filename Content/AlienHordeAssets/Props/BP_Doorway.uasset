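; BP_Doorway is a doorway prop with a door that sits open or closed according to the IsOpened flag.
; BeginPlay reads the flag and calls Open or Close, each snapping Door to a fixed world rotation with no animation, independent of the actor's placed orientation.
; Close also enables query and physics collision on Door, while Open leaves collision untouched.
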(event EventBeginPlay
  (if (Variables|Default|GetIsOpened)
    (CallFunction|Open)
    (else
      (CallFunction|Close))))

(event Collision|EventActorBeginOverlap
  (params (OtherActor :type Actor%20Object%20Reference)))

(event EventTick
  (params (DeltaSeconds :type Float%20%28single-precision%29)))

(fn ConstructionScript)

(fn Open
  (Transformation|SetWorldRotation (Variables|Default|GetDoor) "0.000000,180.000000,0.000000" false false))

(fn Close
  (Transformation|SetWorldRotation (Variables|Default|GetDoor) "0.000000,90.000000,0.000000" false false)
  (Collision|SetCollisionEnabled (Variables|Default|GetDoor) "QueryAndPhysics"))