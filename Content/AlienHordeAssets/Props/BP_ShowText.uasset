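; BP_ShowText is a prop with a box trigger that flags when the player character is near an interactable.
; Box overlaps set InteractableNear on BP_PlayerCharacter, and leaving also removes a widget and clears WIdgetAdded after a short delay.
; The text display is unfinished: the entry branch on WIdgetAdded does nothing, no widget is created here, and the node setting that flag true is disconnected.
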(event OnComponentBeginOverlap(Box)
  (params (OverlappedComponent :type Primitive%20Component%20Object%20Reference) (OtherActor :type Actor%20Object%20Reference) (OtherComp :type Primitive%20Component%20Object%20Reference) (OtherBodyIndex :type Integer) (bFromSweep :type Boolean) (SweepResult :type Hit%20Result%20Structure%20%28by%20ref%29))
  (bind _asbp_player_character (Utilities|Casting|CastToBP_PlayerCharacter OtherActor))
  (Variables|/Game/AlienHordeAssets/Player/Blueprints/BP_PlayerCharacter.BP_PlayerCharacter_C|SetInteractableNear _asbp_player_character true)
  (if (Variables|Default|GetWIdgetAdded)
    _))

(event OnComponentEndOverlap(Box)
  (params (OverlappedComponent :type Primitive%20Component%20Object%20Reference) (OtherActor :type Actor%20Object%20Reference) (OtherComp :type Primitive%20Component%20Object%20Reference) (OtherBodyIndex :type Integer))
  (bind _asbp_player_character (Utilities|Casting|CastToBP_PlayerCharacter OtherActor))
  (Variables|/Game/AlienHordeAssets/Player/Blueprints/BP_PlayerCharacter.BP_PlayerCharacter_C|SetInteractableNear _asbp_player_character false)
  (Widget|RemovefromParent (Variables|Default|GetWidget))
  (Utilities|FlowControl|Delay 0.5)
  (Variables|Default|SetWIdgetAdded false))

(fn ConstructionScript)