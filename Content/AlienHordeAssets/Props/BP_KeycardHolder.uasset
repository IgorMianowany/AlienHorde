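; BP_KeycardHolder is an interactable prop the player searches to find the warehouse keycard.
; Each first interaction increments a counter on the player, granting the keycard with a pickup sound when it equals NumberOfTries, so the card comes from the Nth holder searched rather than a fixed one.
; Tick toggles custom depth on the skeletal mesh as a proximity highlight until the holder is used or the player has the card.
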(event EventBeginPlay
  (bind _asbp_player_character (Utilities|Casting|CastToBP_PlayerCharacter (Game|GetPlayerCharacter 0)))
  (Variables|Default|SetPlayer _asbp_player_character))

(event EventTick
  (params (DeltaSeconds :type Float%20%28single-precision%29))
  (if (or (Variables|/Game/AlienHordeAssets/Player/Blueprints/BP_PlayerCharacter.BP_PlayerCharacter_C|GetHasWarehouseKeycard (Variables|Default|GetPlayer)) (Variables|Default|GetInteracted))
    (Variables|Default|SetInteracted true)
    (Rendering|SetRenderCustomDepth (Variables|Default|GetSkeletalMesh) false)
    (else
      (Rendering|SetRenderCustomDepth (Variables|Default|GetSkeletalMesh) (< (Math|Vector|Distance(Vector) (Transformation|GetActorLocation (Variables|Default|GetPlayer)) (Transformation|GetWorldLocation (Variables|Default|GetSkeletalMesh))) 5e+02)))))

(fn ConstructionScript)

(fn Interact
  (params (Player :type BP%20Player%20Character%20Object%20Reference))
  (Variables|/Game/AlienHordeAssets/Player/Blueprints/BP_PlayerCharacter.BP_PlayerCharacter_C|SetInteractableNear Player false)
  (if (not (Variables|Default|GetInteracted))
    (bind _result (Math|Integer|IncrementInt (Variables|/Game/AlienHordeAssets/Player/Blueprints/BP_PlayerCharacter.BP_PlayerCharacter_C|GetWarehouseKeycardCounter Player))
      (:%20%20
        (bind _output_get (Variables|/Game/AlienHordeAssets/Player/Blueprints/BP_PlayerCharacter.BP_PlayerCharacter_C|SetWarehouseKeycardCounter Player _result))
        (Variables|Default|SetInteracted true)
        (if (== _output_get (Variables|Default|GetNumberOfTries))
          (Variables|/Game/AlienHordeAssets/Player/Blueprints/BP_PlayerCharacter.BP_PlayerCharacter_C|SetHasWarehouseKeycard Player true)
          (Audio|PlaySound2D "/Game/AlienHordeAssets/Props/Audio/item-pickup-37089.item-pickup-37089" 1.0 1.0 0.0 0 0))))))