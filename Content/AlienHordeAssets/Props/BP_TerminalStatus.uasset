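; Terminal status prop that shows whether the player has picked up a key, switching between an open and a closed display.
; On BeginPlay it caches player 0 as BP_PlayerCharacter.
; Every Tick it polls the player's HasKey flag and toggles visibility of the Opened and Closed components, including their children.
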(event EventBeginPlay
  (bind _asbp_player_character (Utilities|Casting|CastToBP_PlayerCharacter (Game|GetPlayerCharacter 0)))
  (Variables|Default|SetPlayer _asbp_player_character))

(event Collision|EventActorBeginOverlap
  (params (OtherActor :type Actor%20Object%20Reference)))

(event EventTick
  (params (DeltaSeconds :type Float%20%28single-precision%29))
  (if (Variables|/Game/AlienHordeAssets/Player/Blueprints/BP_PlayerCharacter.BP_PlayerCharacter_C|GetHasKey (Variables|Default|GetPlayer))
    (Rendering|SetVisibility (Variables|Default|GetOpened) true true)
    (Rendering|SetVisibility (Variables|Default|GetClosed) false true)
    (else
      (Rendering|SetVisibility (Variables|Default|GetClosed) true true)
      (Rendering|SetVisibility (Variables|Default|GetOpened) false true))))

(fn ConstructionScript)