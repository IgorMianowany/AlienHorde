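; BP_KeycardHolderInteract is a keycard holder prop that toggles custom depth on its skeletal mesh according to the player's proximity.
; BeginPlay caches player 0's character as BP_PlayerCharacter.
; Every Tick compares that character's distance to the mesh against a fixed threshold and enables custom depth rendering while in range.
; The graph contains no interaction logic beyond this proximity check.
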(event EventBeginPlay
  (bind _asbp_player_character (Utilities|Casting|CastToBP_PlayerCharacter (Game|GetPlayerCharacter 0)))
  (Variables|Default|SetPlayer _asbp_player_character))

(event EventTick
  (params (DeltaSeconds :type Float%20%28single-precision%29))
  (Rendering|SetRenderCustomDepth (Variables|Default|GetSkeletalMesh) (< (Math|Vector|Distance(Vector) (Transformation|GetActorLocation (Variables|Default|GetPlayer)) (Transformation|GetWorldLocation (Variables|Default|GetSkeletalMesh))) 5e+02)))

(fn ConstructionScript)