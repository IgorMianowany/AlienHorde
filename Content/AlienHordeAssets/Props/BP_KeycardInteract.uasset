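; BP_KeycardInteract is an interactable keycard prop that shows and hides an on-screen info widget.
; Its Interact function toggles on the Interacted flag, either creating a W_KeycardInfo widget and adding it to the viewport, or removing the stored widget.
; The event graph holds only disabled default events, so all of the behavior lives in Interact.
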(event EventBeginPlay)

(event Collision|EventActorBeginOverlap
  (params (OtherActor :type Actor%20Object%20Reference)))

(event EventTick
  (params (DeltaSeconds :type Float%20%28single-precision%29)))

(fn ConstructionScript
  (|CallParentFunction))

(fn Interact
  (if (Variables|Default|GetInteracted)
    (Widget|RemovefromParent (Variables|Default|GetWidget))
    (Variables|Default|SetInteracted false)
    (else
      (bind _returnvalue (UserInterface|CreateWidget "/Game/AlienHordeAssets/UI/W_KeycardInfo.W_KeycardInfo_C"))
      (bind _output_get (Variables|Default|SetWidget _returnvalue))
      (UserInterface|Viewport|AddtoViewport _returnvalue 0)
      (Variables|Default|SetInteracted true))))