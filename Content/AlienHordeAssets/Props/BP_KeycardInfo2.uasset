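; BP_KeycardInfo2 is a keycard info pickup prop that grants the player the room key and records the second info card as found.
; Its construction script runs the parent's, then sets WidgetClass to W_KeycardInfo2.
; On overlap it runs the parent's handling, then casts the other actor to BP_PlayerCharacter and sets both progress flags on it.
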(event EventBeginPlay
  (|CallParentFunction) ; This node is disabled and will not be called.\nDrag off pins to build functionality.
)

(event Collision|EventActorBeginOverlap
  (params (OtherActor :type Actor%20Object%20Reference))
  (|CallParentFunction OtherActor)
  (bind _asbp_player_character (Utilities|Casting|CastToBP_PlayerCharacter OtherActor))
  (Variables|/Game/AlienHordeAssets/Player/Blueprints/BP_PlayerCharacter.BP_PlayerCharacter_C|SetFoundSecondInfoCard _asbp_player_character true)
  (Variables|/Game/AlienHordeAssets/Player/Blueprints/BP_PlayerCharacter.BP_PlayerCharacter_C|SetHasRoomKey _asbp_player_character true))

(event EventTick
  (params (DeltaSeconds :type Float%20%28single-precision%29))
  (|CallParentFunction DeltaSeconds) ; This node is disabled and will not be called.\nDrag off pins to build functionality.
)

(fn ConstructionScript
  (|CallParentFunction)
  (Variables|Default|SetWidgetClass "/Game/AlienHordeAssets/UI/Info/W_KeycardInfo2.W_KeycardInfo2_C"))