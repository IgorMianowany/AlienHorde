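; Interactable escape info prop that shows the W_EscapeInfo widget on screen.
; The construction script sets the widget class, and Interact toggles the widget, creating a new instance on each open and removing it on the next use.
; Tick removes the widget and resets the toggle once the first player's character is more than 200 units from the static mesh.
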(event EventBeginPlay)

(event Collision|EventActorBeginOverlap
  (params (OtherActor :type Actor%20Object%20Reference)))

(event EventTick
  (params (DeltaSeconds :type Float%20%28single-precision%29))
  (bind _widget (Variables|Default|GetWidget))
  (if (> (Math|Vector|Distance(Vector) (Transformation|GetWorldLocation (Variables|Default|GetStaticMesh)) (Transformation|GetActorLocation (Game|GetPlayerCharacter 0))) 2e+02)
    (Utilities|IsValid _widget
      (:Is%20Valid
        (Widget|RemovefromParent _widget)
        (Variables|Default|SetInteracted false)))))

(fn ConstructionScript
  (|CallParentFunction)
  (Variables|Default|SetWidgetClass "/Game/AlienHordeAssets/UI/Info/W_EscapeInfo.W_EscapeInfo_C"))

(fn Interact
  (params (Player :type BP%20Player%20Character%20Object%20Reference))
  (if (Variables|Default|GetInteracted)
    (Widget|RemovefromParent (Variables|Default|GetWidget))
    (Variables|Default|SetInteracted false)
    (else
      (bind _returnvalue (UserInterface|CreateWidget (Variables|Default|GetWidgetClass)))
      (bind _output_get (Variables|Default|SetWidget _returnvalue))
      (UserInterface|Viewport|AddtoViewport _output_get 0)
      (Variables|Default|SetInteracted true))))