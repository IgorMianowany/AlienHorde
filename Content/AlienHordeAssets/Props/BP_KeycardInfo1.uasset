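; BP_KeycardInfo1 is a keycard info prop that also removes the Behemot from the game when the player overlaps it.
; Its construction script sets the inherited widget class to W_KeycardInfo1 after running the parent's construction.
; On overlap it runs the parent logic, then for a BP_PlayerCharacter destroys the Behemot referenced by BP_GameMode.
; A BehemotDead flag makes the removal happen only once.
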(event EventBeginPlay
  (|CallParentFunction) ; This node is disabled and will not be called.\nDrag off pins to build functionality.
)

(event Collision|EventActorBeginOverlap
  (params (OtherActor :type Actor%20Object%20Reference))
  (|CallParentFunction OtherActor)
  (if (not (Variables|Default|GetBehemotDead))
    (Utilities|Casting|CastToBP_PlayerCharacter OtherActor)
    (bind _asbp_game_mode (Utilities|Casting|CastToBP_GameMode (Game|GetGameMode)))
    (Actor|DestroyActor (Variables|/Game/AlienHordeAssets/Gamemode/BP_GameMode.BP_GameMode_C|GetBehemot _asbp_game_mode))
    (Variables|Default|SetBehemotDead true)))

(event EventTick
  (params (DeltaSeconds :type Float%20%28single-precision%29))
  (|CallParentFunction DeltaSeconds) ; This node is disabled and will not be called.\nDrag off pins to build functionality.
)

(fn ConstructionScript
  (|CallParentFunction)
  (Variables|Default|SetWidgetClass "/Game/AlienHordeAssets/UI/W_KeycardInfo1.W_KeycardInfo1_C"))