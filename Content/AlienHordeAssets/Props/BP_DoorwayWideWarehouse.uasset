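; BP_DoorwayWideWarehouse is a wide warehouse doorway prop whose alarm lights show whether the player can use it.
; BeginPlay caches the BP_PlayerCharacter from player index 0.
; Every tick, it turns both point lights and alarm-light glass materials green when that player has the key and IsLocked is false, and red otherwise.
; The graph contains only this indicator logic, with no door movement.
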(event EventBeginPlay
  (bind _asbp_player_character (Utilities|Casting|CastToBP_PlayerCharacter (Game|GetPlayerCharacter 0)))
  (Variables|Default|SetPlayer _asbp_player_character))

(event Collision|EventActorBeginOverlap
  (params (OtherActor :type Actor%20Object%20Reference)))

(event EventTick
  (params (DeltaSeconds :type Float%20%28single-precision%29))
  (if (and (Variables|/Game/AlienHordeAssets/Player/Blueprints/BP_PlayerCharacter.BP_PlayerCharacter_C|GetHasKey (Variables|Default|GetPlayer)) (not (Variables|Default|GetIsLocked)))
    (Rendering|Components|Light|SetLightColor (Variables|Default|GetPointLight2) "(R=0.000000,G=1.000000,B=0.018193,A=1.000000)" true)
    (Rendering|Material|SetMaterial (Variables|Default|GetSM_AlarmLight1) 0 "/Game/ModSci_EngiProps/Materials/AlarmLight/M_AlarmLightGreen_Glass.M_AlarmLightGreen_Glass")
    (else
      (Rendering|Components|Light|SetLightColor (Variables|Default|GetPointLight2) "(R=1.000000,G=0.016990,B=0.000000,A=1.000000)" true)
      (Rendering|Material|SetMaterial (Variables|Default|GetSM_AlarmLight1) 0 "/Game/ModSci_EngiProps/Materials/AlarmLight/M_AlarmLight_Glass.M_AlarmLight_Glass"))))

(fn ConstructionScript)