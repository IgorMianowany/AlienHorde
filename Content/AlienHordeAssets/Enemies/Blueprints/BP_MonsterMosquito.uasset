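; BP_MonsterMosquito is a mosquito enemy Blueprint that adds a death adjustment for its raised mesh to parent class behavior.
; Tick calls the parent, then, while IsDead is true, runs a short Delay and lowers the Mesh's relative location so the corpse does not float.
; The check stays on Tick with no one-shot guard, so the reposition repeats after each delay.
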(event EventBeginPlay
  (|CallParentFunction) ; This node is disabled and will not be called.\nDrag off pins to build functionality.
)

(event Collision|EventActorBeginOverlap
  (params (OtherActor :type Actor%20Object%20Reference))
  (|CallParentFunction OtherActor) ; This node is disabled and will not be called.\nDrag off pins to build functionality.
)

(event EventTick
  (params (DeltaSeconds :type Float%20%28single-precision%29))
  (|CallParentFunction DeltaSeconds)
  ;[1 1 1] Mosquito model needs to be higher so after death we need to bring it down to avoid the mesh floating in the air
  (if (Variables|Default|GetIsDead)
    (Utilities|FlowControl|Delay 0.4)
    (Transformation|SetRelativeLocation (Variables|Character|GetMesh) "0.000000,0.000000,-100.000000" false false)))

(fn ConstructionScript
  (|CallParentFunction))