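; Parent monster enemy that patrols, chases the player and melee attacks, with a floating health readout turned to the player's spring arm yaw.
; A timeline lerps AI move targets for patrol until sight, damage or OnSpawn triggers pursuit.
; Attack hitbox overlaps start delayed, timer-repeated hits that damage and knock back the player.
; TakeDamage massively widens PawnSensing range, updates health and on death sets IsDead, disabling collision and hiding the readout.
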(event OnComponentBeginOverlap(AttackHitbox)
  (params (OverlappedComponent :type Primitive%20Component%20Object%20Reference) (OtherActor :type Actor%20Object%20Reference) (OtherComp :type Primitive%20Component%20Object%20Reference) (OtherBodyIndex :type Integer) (bFromSweep :type Boolean) (SweepResult :type Hit%20Result%20Structure%20%28by%20ref%29))
  ;[1 1 1] Run at Player Events
  (Utilities|Casting|CastToBP_PlayerCharacter OtherActor)
  (Variables|Default|SetIsPlayerInRange true)
  (Utilities|Time|SetTimerbyEvent (delegate Custom|Attack%20Cooldown) (Variables|Default|GetAttackSpeed) true true)
  (Variables|Default|SetIsAttacking true)
  (Utilities|FlowControl|Delay 0.3)
  (CallFunction|Attack OtherActor OtherComp)
  (if (Variables|Default|GetIsAttacking)
    (Utilities|FlowControl|Delay 0.3)
    (Variables|Default|SetIsAttacking false)))

(event OnComponentBeginOverlap(Hitbox)
  (params (OverlappedComponent :type Primitive%20Component%20Object%20Reference) (OtherActor :type Actor%20Object%20Reference) (OtherComp :type Primitive%20Component%20Object%20Reference) (OtherBodyIndex :type Integer) (bFromSweep :type Boolean) (SweepResult :type Hit%20Result%20Structure%20%28by%20ref%29))
  (Utilities|Casting|CastToBP_PlayerCharacter OtherActor))

(event OnComponentEndOverlap(AttackHitbox)
  (params (OverlappedComponent :type Primitive%20Component%20Object%20Reference) (OtherActor :type Actor%20Object%20Reference) (OtherComp :type Primitive%20Component%20Object%20Reference) (OtherBodyIndex :type Integer))
  ;[1 1 1] Run at Player Events
  (Utilities|Casting|CastToBP_PlayerCharacter OtherActor)
  (Variables|Default|SetIsPlayerInRange false))

(event OnComponentBeginOverlap(AttackHitbox1)
  (params (OverlappedComponent :type Primitive%20Component%20Object%20Reference) (OtherActor :type Actor%20Object%20Reference) (OtherComp :type Primitive%20Component%20Object%20Reference) (OtherBodyIndex :type Integer) (bFromSweep :type Boolean) (SweepResult :type Hit%20Result%20Structure%20%28by%20ref%29))
  ;[1 1 1] Run at Player Events
  (Utilities|Casting|CastToBP_PlayerCharacter (stale OnComponentBeginOverlap(AttackHitbox) OtherActor))
  (Variables|Default|SetIsPlayerInRange true)
  (Utilities|Time|SetTimerbyEvent (delegate Custom|Attack%20Cooldown) (Variables|Default|GetAttackSpeed) true true)
  (Variables|Default|SetIsAttacking true)
  (Utilities|FlowControl|Delay 0.3)
  (CallFunction|Attack (stale OnComponentBeginOverlap(AttackHitbox) OtherActor) (stale OnComponentBeginOverlap(AttackHitbox) OtherComp))
  (if (Variables|Default|GetIsAttacking)
    (Utilities|FlowControl|Delay 0.3)
    (Variables|Default|SetIsAttacking false)))

(event OnSeePawn(PawnSensing)
  (params (Pawn :type Pawn%20Object%20Reference))
  ;[1 1 1] Run at Player Events
  (Variables|Default|SetShouldPatrol false)
  (CallFunction|RunatPlayer (Game|Player|GetPlayerPawn 0)))

(event OnComponentEndOverlap(AttackHitbox1)
  (params (OverlappedComponent :type Primitive%20Component%20Object%20Reference) (OtherActor :type Actor%20Object%20Reference) (OtherComp :type Primitive%20Component%20Object%20Reference) (OtherBodyIndex :type Integer))
  ;[1 1 1] Run at Player Events
  (Utilities|Casting|CastToBP_PlayerCharacter (stale OnComponentEndOverlap(AttackHitbox) OtherActor))
  (Variables|Default|SetIsPlayerInRange false))

(event Custom|On%20Spawn
  ;[1 1 1] Run at Player Events
  (Variables|Default|SetShouldPatrol false)
  (CallFunction|RunatPlayer (Game|Player|GetPlayerPawn 0)))

(event Custom|Event%20AfterTakeDamage
  ;[1 1 1] Run at Player Events
  (Utilities|FlowControl|Delay 0.3)
  (Variables|Default|SetIsHit false))

(event Custom|Attack%20Cooldown
  ;[1 1 1] Run at Player Events
  (if (Variables|Default|GetIsPlayerInRange)
    (Variables|Default|SetIsAttacking true)
    (Utilities|FlowControl|Delay 0.3)
    (CallFunction|Attack (stale OnComponentBeginOverlap(AttackHitbox) OtherActor) (stale OnComponentBeginOverlap(AttackHitbox) OtherComp))
    (if (Variables|Default|GetIsAttacking)
      (Utilities|FlowControl|Delay 0.3)
      (Variables|Default|SetIsAttacking false))))

(event Custom|Event%20TakeDamage
  ;[1 1 1] Run at Player Events
  (Variables|Default|SetShouldPatrol false)
  (CallFunction|RunatPlayer (Game|Player|GetPlayerPawn 0)))

(event Collision|EventActorBeginOverlap
  (params (OtherActor :type Actor%20Object%20Reference))
  (Utilities|Casting|CastToBP_Bullet OtherActor))

(event EventTick
  (params (DeltaSeconds :type Float%20%28single-precision%29))
  (if (Variables|Default|GetCanSeePlayer)
    (CallFunction|RunatPlayer (Game|Player|GetPlayerPawn 0)))
  ;[1 1 1] Patrol movement
  (CallFunction|RotateHealthDisplay)
  (if (Variables|Default|GetCanSeePlayer)
    (Utilities|FlowControl|DoOnce false
      (:Completed
        (bind _patrol_track (Timeline|Timeline Stop)
          (:Update
            (if (Variables|Default|GetShouldPatrol)
              (AI|Navigation|MovetoLocation (AI|GetAIController self) (Math|Vector|Lerp(Vector) (stale EventBeginPlay _output_get) (stale EventBeginPlay _output_get_2) _patrol_track) -1.0 true true false true 0))))))))

(event EventBeginPlay
  (bind _returnvalue (Transformation|GetActorLocation))
  (Variables|/Script/Engine.CharacterMovementComponent|SetMaxWalkSpeed (Variables|Character|GetCharacterMovement) (Variables|Default|GetSpeed))
  (CallFunction|SetAggroRange (Variables|Default|GetAggroRange))
  ;[1 1 1] Patrol movement
  (Rendering|Components|TextRender|SetText (Variables|Default|GetHealth%20Display) (Utilities|Text|ToText(Float) (Variables|Default|GetHealth%20Points) "HalfToEven"))
  (bind _output_get (Variables|Default|SetStart (+ _returnvalue (* "-500.000000,500.000000,0.000000" (Math|Random|RandomIntegerinRange -1 1)))))
  (bind _output_get_2 (Variables|Default|SetEnd (+ _returnvalue "500.000000,0.000000,0.000000")))
  (bind _patrol_track (Timeline|Timeline PlayFromStart)
    (:Update
      (if (Variables|Default|GetShouldPatrol)
        (AI|Navigation|MovetoLocation (AI|GetAIController self) (Math|Vector|Lerp(Vector) _output_get _output_get_2 _patrol_track) -1.0 true true false true 0)))))

(fn ConstructionScript)

(fn TakeDamage
  (params (Damage :type Float%20%28double-precision%29))
  (if (not (Variables|Default|GetIsDead))
    (CallFunction|SetAggroRange 1e+05)
    (Variables|Default|SetIsHit true)
    (bind _output_get (Variables|Default|SetHealth%20Points (- (Variables|Default|GetHealth%20Points) Damage)))
    (Rendering|Components|TextRender|SetText (Variables|Default|GetHealth%20Display) (Utilities|Text|ToText(Float) (Variables|Default|GetHealth%20Points) "HalfToEven"))
    (CallFunction|EventTakeDamage)
    (CallFunction|EventAfterTakeDamage)
    (if (<= _output_get 0.0)
      (Utilities|FlowControl|DoOnce false
        (:Completed
          (Variables|Default|SetIsDead true)
          (Collision|SetActorEnableCollision false)
          (Rendering|SetVisibility (Variables|Default|GetHealth%20Display) false false))))))

(fn RunatPlayer
  (params (Player :type Pawn%20Object%20Reference))
  (bind _asbp_player_character (Utilities|Casting|CastToBP_PlayerCharacter Player))
  (Variables|Default|SetCanSeePlayer true)
  (if (and (not (Variables|Default|GetIsDead)) (Variables|Default|GetShouldRunAtPlayer))
    (bind _returnvalue (AI|Navigation|MovetoActor (AI|GetAIController self) _asbp_player_character -1.0 false true false "/Script/AIModule.NavFilter_AIControllerDefault"))
    (Development|PrintString (Utilities|String|EnumtoString _returnvalue))
    (else
      (Pawn|Components|CharacterMovement|DisableMovement (Variables|Character|GetCharacterMovement))
      (Collision|SetCollisionEnabled (Variables|Collision|GetCapsuleComponent) "NoCollision"))))

(fn Attack
  (params (Player%20Actor :type Actor%20Object%20Reference) (Component :type Primitive%20Component%20Object%20Reference))
  (if (and (Variables|Default|GetIsPlayerInRange) (not (Variables|Default|GetIsDead)))
    (bind _asbp_player_character (Utilities|Casting|CastToBP_PlayerCharacter (Game|GetPlayerCharacter 0)))
    (Variables|Default|SetIsAttacking true)
    (Default|TakeDamage _asbp_player_character (Variables|Default|GetAttackDamage))
    (Default|KnockBack _asbp_player_character (* (Math|Vector|GetForwardVector (Transformation|GetWorldRotation (Variables|Collision|GetCapsuleComponent))) 1e+03))))

(fn Patrol
  (bind _output_get (Variables|Default|SetStart (* "-500.000000,500.000000,0.000000" (Math|Random|RandomIntegerinRange -1 1))))
  (bind _output_get_2 (Variables|Default|SetEnd (+ (Transformation|GetActorLocation) "500.000000,0.000000,0.000000" ""))))

(fn SetAggroRange
  (params (Range :type Float%20%28double-precision%29))
  (bind _pawnsensing (Variables|Default|GetPawnSensing))
  (bind _output_get (Variables|/Script/AIModule.PawnSensingComponent|SetHearingThreshold _pawnsensing Range))
  (bind _output_get_2 (Variables|/Script/AIModule.PawnSensingComponent|SetLOSHearingThreshold _pawnsensing _output_get))
  (Variables|/Script/AIModule.PawnSensingComponent|SetSightRadius _pawnsensing _output_get_2))

(fn RotateHealthDisplay
  (bind _asbp_player_character (Utilities|Casting|CastToBP_PlayerCharacter (Game|GetPlayerCharacter 0)))
  (Transformation|SetWorldRotation (Variables|Default|GetHealth%20Display) (Math|Rotator|MakeRotator 1.8e+02 9e+01 (.yaw (Transformation|GetWorldRotation (Variables|/Game/AlienHordeAssets/Player/Blueprints/BP_PlayerCharacter.BP_PlayerCharacter_C|GetSpringArm _asbp_player_character)))) false false))

(fn LookatPlayer
  (bind _capsulecomponent (Variables|Collision|GetCapsuleComponent))
  (Transformation|SetWorldRotation _capsulecomponent (Math|Rotator|FindLookatRotation (Transformation|GetWorldLocation _capsulecomponent) (Transformation|GetWorldLocation (Variables|/Script/Engine.Character|GetMesh (Game|GetPlayerCharacter 0)))) false false))

(fn SetHealth
  (params (Health :type Float%20%28double-precision%29))
  (Variables|Default|SetHealth%20Points Health))