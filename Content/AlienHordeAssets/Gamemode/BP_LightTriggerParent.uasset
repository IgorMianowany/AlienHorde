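; BP_LightTriggerParent is a parent trigger actor that lights up a set of rect lights, apparently corridor lights, when the player enters it.
; On BeginPlay it gathers every RectLight whose display name matches LightDisplayName into the CorridorLight array.
; The first overlap by BP_PlayerCharacter passes a DoOnce and sets a fixed intensity on each stored light, with no logic to switch them back.
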(event EventBeginPlay
  (bind _outactors (Actor|GetAllActorsOfClass "/Script/Engine.RectLight"))
  (for _array_element _outactors
    (if (Utilities|Enum|Equal(Enum) (Utilities|GetDisplayName _array_element) (Variables|Default|GetLightDisplayName))
      (Utilities|Array|Add (Variables|Default|GetCorridorLight) _array_element))))

(event Collision|EventActorBeginOverlap
  (params (OtherActor :type Actor%20Object%20Reference))
  (Utilities|Casting|CastToBP_PlayerCharacter OtherActor)
  (Utilities|FlowControl|DoOnce false
    (:Completed
      (for _array_element (Variables|Default|GetCorridorLight)
        (Rendering|Components|Light|SetIntensity (Variables|/Script/Engine.RectLight|GetRectLightComponent _array_element) 8.0)))))

(event EventTick
  (params (DeltaSeconds :type Float%20%28single-precision%29)))

(fn ConstructionScript)