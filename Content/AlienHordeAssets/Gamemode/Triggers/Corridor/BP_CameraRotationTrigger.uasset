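; Corridor trigger volume that switches the player's camera between two orientations each time BP_PlayerCharacter enters it.
; On begin overlap it reads the player's CameraAngle to choose between one or three EventRotateCamera calls, then sets CameraAngle to the opposite preset.
; An IsTriggered flag tracks the overlap and drives a debug print on Tick; exiting only clears the flag.
; A duplicate copy of the rotation logic is left unconnected.
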(event OnComponentBeginOverlap(CollisionComponent)
  (params (OverlappedComponent :type Primitive%20Component%20Object%20Reference) (OtherActor :type Actor%20Object%20Reference) (OtherComp :type Primitive%20Component%20Object%20Reference) (OtherBodyIndex :type Integer) (bFromSweep :type Boolean) (SweepResult :type Hit%20Result%20Structure%20%28by%20ref%29))
  (bind _asbp_player_character (Utilities|Casting|CastToBP_PlayerCharacter OtherActor))
  (Variables|Default|SetPlayer _asbp_player_character)
  (Variables|Default|SetIsTriggered true)
  (if (< (Variables|/Game/AlienHordeAssets/Player/Blueprints/BP_PlayerCharacter.BP_PlayerCharacter_C|GetCameraAngle (Variables|Default|GetPlayer)) -5e+01)
    (Default|EventRotateCamera (Variables|Default|GetPlayer))
    (Default|EventRotateCamera (Variables|Default|GetPlayer))
    (Default|EventRotateCamera (Variables|Default|GetPlayer))
    (Variables|/Game/AlienHordeAssets/Player/Blueprints/BP_PlayerCharacter.BP_PlayerCharacter_C|SetCameraAngle (Variables|Default|GetPlayer) -25.0)
    (else
      (Default|EventRotateCamera (Variables|Default|GetPlayer))
      (Variables|/Game/AlienHordeAssets/Player/Blueprints/BP_PlayerCharacter.BP_PlayerCharacter_C|SetCameraAngle (Variables|Default|GetPlayer) -55.0))))

(event OnComponentEndOverlap(CollisionComponent)
  (params (OverlappedComponent :type Primitive%20Component%20Object%20Reference) (OtherActor :type Actor%20Object%20Reference) (OtherComp :type Primitive%20Component%20Object%20Reference) (OtherBodyIndex :type Integer))
  (Utilities|Casting|CastToBP_PlayerCharacter OtherActor)
  (Variables|Default|SetIsTriggered false))

(event Collision|EventActorBeginOverlap
  (params (OtherActor :type Actor%20Object%20Reference)))

(event EventTick
  (params (DeltaSeconds :type Float%20%28single-precision%29))
  (if (Variables|Default|GetIsTriggered)
    (Development|PrintString "Hello" true true "(R=0.000000,G=0.660000,B=1.000000,A=1.000000)" 0.1)))

(fn ConstructionScript)