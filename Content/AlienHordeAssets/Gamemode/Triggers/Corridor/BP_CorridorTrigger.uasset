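; BP_CorridorTrigger is a key pickup trigger that sets off an explosion through the game mode.
; When a BP_PlayerCharacter overlaps it, the trigger sets that player's HasKey flag.
; A DoOnce then destroys the key's root and cube components and, after a short delay, calls TriggerExplosion on BP_GameMode.
; The actor itself remains, so only the removal and explosion are limited to one run.
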(event EventBeginPlay)

(event Collision|EventActorBeginOverlap
  (params (OtherActor :type Actor%20Object%20Reference))
  (bind _asbp_player_character (Utilities|Casting|CastToBP_PlayerCharacter OtherActor))
  (Variables|/Game/AlienHordeAssets/Player/Blueprints/BP_PlayerCharacter.BP_PlayerCharacter_C|SetHasKey _asbp_player_character true)
  (Utilities|FlowControl|DoOnce false
    (:Completed
      (Components|DestroyComponent (Variables|Default|GetKeyRoot))
      (bind _asbp_game_mode (Utilities|Casting|CastToBP_GameMode (Game|GetGameMode)))
      (Utilities|FlowControl|Delay 1.0)
      (Default|TriggerExplosion _asbp_game_mode))))

(event EventTick
  (params (DeltaSeconds :type Float%20%28single-precision%29)))

(fn ConstructionScript)