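; BP_CameraControlTutorial is a tutorial trigger for camera controls that supplies its own widget to inherited trigger logic.
; On BeginPlay it creates a W_CameraTutorial widget and stores it in the Widget variable.
; On overlap it runs the parent's overlap handling only if player 0's BP_PlayerCharacter has found the second info card, without itself checking which actor overlapped.
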(event EventBeginPlay
  (|CallParentFunction)
  (bind _returnvalue (UserInterface|CreateWidget "/Game/AlienHordeAssets/UI/Tutorials/W_CameraTutorial.W_CameraTutorial_C"))
  (Variables|Default|SetWidget _returnvalue))

(event Collision|EventActorBeginOverlap
  (params (OtherActor :type Actor%20Object%20Reference))
  (bind _asbp_player_character (Utilities|Casting|CastToBP_PlayerCharacter (Game|GetPlayerCharacter 0)))
  (if (Variables|/Game/AlienHordeAssets/Player/Blueprints/BP_PlayerCharacter.BP_PlayerCharacter_C|GetFoundSecondInfoCard _asbp_player_character)
    (|CallParentFunction OtherActor)))

(event EventTick
  (params (DeltaSeconds :type Float%20%28single-precision%29))
  (|CallParentFunction DeltaSeconds))

(fn ConstructionScript
  (|CallParentFunction))