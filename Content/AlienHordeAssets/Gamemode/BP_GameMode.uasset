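; Game mode that runs the scripted events of an Alien Horde level, including doors, enemy spawns, weapon spotlight and an explosion that releases a Beholder.
; BeginPlay caches level actors, picking out specific lights by display name, as is done later for doorways.
; The arena fight shuts its doors, turns the light red and spawns mosquitoes on a looping timer up to a limit.
; Tick moves that light with the player and prunes dead enemies, triggering cleanup.
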(event Custom|Event%20TriggerEnemySpawn
  (CallFunction|TriggerEnemySpawn))

(event Custom|Event%20StartArenaFight
  ;[1 1 1] Arena Fight
  (CallFunction|CloseAllArenaFightDoors)
  (Utilities|FlowControl|Delay 1.0)
  (Variables|Default|SetArenaFightInProgress true)
  (CallFunction|ArenaFightSetLighting)
  (bind _returnvalue (Utilities|Time|SetTimerbyEvent (delegate Custom|SpawnMosquito) (Variables|Default|GetArenaFightSpawnCooldown) true)))

(event Custom|AllArenaEnemiesDead
  ;[1 1 1] Arena Fight
  (if (and (> (Variables|Default|GetArenaFightCounter) (Variables|Default|GetArenaCounterLimit)) (Utilities|Array|IsEmpty (Variables|Default|GetArenaFIghtEnemies)))
    (Utilities|FlowControl|Delay (Variables|Default|GetArenaFightSpawnCooldown))
    (CallFunction|ArenaFightCleanup)))

(event Custom|SpawnMosquito
  ;[1 1 1] Arena Fight
  (Math|Integer|IncrementInt (Variables|Default|GetArenaFightCounter)
    (:%20%20
      (bind _location (CallFunction|ArenaFightGetRandomSpawn))
      (bind _returnvalue (Game|SpawnActorfromClass "/Game/AlienHordeAssets/Enemies/Blueprints/BP_MonsterMosquito.BP_MonsterMosquito_C" _location "AlwaysSpawn" "MultiplyWithRoot" 0 0))
      (Default|OnSpawn _returnvalue)
      (Utilities|Array|Add (Variables|Default|GetArenaFIghtEnemies) _returnvalue)
      (Variables|Default|SetAreAllArenaFightEnemiesDead true)
      (if (> (Variables|Default|GetArenaFightCounter) (Variables|Default|GetArenaCounterLimit))
        (Utilities|Time|ClearandInvalidateTimerbyHandle (stale Custom|Event%20StartArenaFight _returnvalue))))))

(event EventBeginPlay
  ;[1 1 1] Setup
  (bind _asbp_player_character (Utilities|Casting|CastToBP_PlayerCharacter (Game|GetPlayerCharacter 0)))
  (Variables|Default|SetPlayer _asbp_player_character)
  (bind _outactors (Actor|GetAllActorsOfClass "/Game/AlienHordeAssets/Props/BP_Doorway.BP_Doorway_C"))
  (Variables|Default|SetDoorways _outactors)
  (bind _outactors_2 (Actor|GetAllActorsOfClass "/Game/AlienHordeAssets/Gamemode/Triggers/Corridor/BP_ExplosionSpawn.BP_ExplosionSpawn_C"))
  (Variables|Default|SetExplosionSpawn (.OutItem (Utilities|Array|Random _outactors_2)))
  (bind _outactors_3 (Actor|GetAllActorsOfClass "/Script/Engine.SpotLight"))
  (for _array_element _outactors_3
    (if (Utilities|Enum|Equal(Enum) (Utilities|GetDisplayName _array_element) "WeaponSpotlight")
      (bind _asspot_light (Utilities|Casting|CastToSpotLight _array_element))
      (Variables|Default|SetFIrstWeaponSpotlight _asspot_light)
      (bind _outactors_4 (Actor|GetAllActorsOfClass "/Game/AlienHordeAssets/Enemies/Blueprints/BP_EnemySpawn.BP_EnemySpawn_C"))
      (Variables|Default|SetSpawnPoints _outactors_4)
      (bind _outactors_5 (Actor|GetAllActorsOfClass "/Script/Engine.PointLight"))
      (for _array_element_2 _outactors_5
        (if (Utilities|Enum|Equal(Enum) (Utilities|GetDisplayName _array_element_2) "ArenaLight")
          (bind _output_get (Variables|Default|SetArenaLight _array_element_2))
          (Variables|Default|SetArenaFightStartingLightPosition (Transformation|GetWorldLocation (Variables|/Script/Engine.Actor|GetRootComponent _output_get)))))))
  (bind _outactors_6 (Actor|GetAllActorsOfClass "/Game/AlienHordeAssets/Enemies/Blueprints/BP_EnemySpawn.BP_EnemySpawn_C"))
  (Variables|Default|SetSpawnPoints _outactors_6)
  (bind _outactors_7 (Actor|GetAllActorsOfClass "/Script/Engine.PointLight"))
  (for _array_element_3 _outactors_7
    (if (Utilities|Enum|Equal(Enum) (Utilities|GetDisplayName _array_element_3) "ArenaLight")
      (bind _output_get_2 (Variables|Default|SetArenaLight _array_element_3))
      (Variables|Default|SetArenaFightStartingLightPosition (Transformation|GetWorldLocation (Variables|/Script/Engine.Actor|GetRootComponent _output_get_2))))))

(event EventTick
  (params (DeltaSeconds :type Float%20%28single-precision%29))
  ;[1 0 0] Event tick
  (CallFunction|ArenaFightUpdate))

(fn ConstructionScript)

(fn TriggerEnemySpawn
  (for _array_element (Variables|Default|GetSpawnPoints)
    (Utilities|FlowControl|DoOnce false
      (:Completed
        (bind _returnvalue (Game|SpawnActorfromClass "/Game/AlienHordeAssets/Enemies/Blueprints/BP_MonsterParent.BP_MonsterParent_C" (Transformation|GetActorTransform _array_element) "AlwaysSpawn" "MultiplyWithRoot" 0 0))
        (Default|OnSpawn _returnvalue)))))

(fn StartArenaFight
  (while true
    (Utilities|Time|SetTimerbyFunctionName 0 "" 0.0)))

(fn CloseAllArenaFightDoors
  (for _array_element (Variables|Default|GetDoorways)
    (if (Utilities|Enum|Equal(Enum) (Utilities|GetDisplayName _array_element) "ArenaFightDoorway")
      (Utilities|Array|Add (Variables|Default|GetArenaFightDoorways) _array_element)
      (Default|Close _array_element))))

(fn ArenaFightSetLighting
  (bind _arenalight (Variables|Default|GetArenaLight))
  (bind _lightcomponent (Variables|/Script/Engine.Light|GetLightComponent _arenalight))
  (Rendering|Components|Light|SetLightColor _lightcomponent "(R=0.703125,G=0.000000,B=0.003663,A=1.000000)" true)
  (Rendering|Components|Light|SetIntensity _lightcomponent 1.6e+02)
  (Variables|/Game/AlienHordeAssets/Player/Blueprints/BP_PlayerCharacter.BP_PlayerCharacter_C|SetIsDarkMode (Variables|Default|GetPlayer) true))

(fn ArenaFightGetRandomSpawn
  (return (Transformation|GetActorTransform (.OutItem (Utilities|Array|Random (Variables|Default|GetSpawnPoints))))))

(fn ArenaFightCleanup
  (bind _arenalight (Variables|Default|GetArenaLight))
  (bind _lightcomponent (Variables|/Script/Engine.Light|GetLightComponent _arenalight))
  (Variables|Default|SetArenaFightInProgress false)
  (Rendering|Components|Light|SetLightColor _lightcomponent "(R=0.703125,G=0.703125,B=0.703125,A=1.000000)" true)
  (Rendering|Components|Light|SetIntensity _lightcomponent 1e+02)
  (Transformation|SetWorldLocation (Variables|/Script/Engine.Actor|GetRootComponent _arenalight) (Variables|Default|GetArenaFightStartingLightPosition) false false)
  (Variables|/Game/AlienHordeAssets/Player/Blueprints/BP_PlayerCharacter.BP_PlayerCharacter_C|SetIsDarkMode (Variables|Default|GetPlayer) false)
  (for _array_element (Variables|Default|GetArenaFightDoorways)
    (Default|Open _array_element)))

(fn ArenaFightUpdate
  (bind _arenafightenemies (Variables|Default|GetArenaFIghtEnemies))
  (bind _arenalight (Variables|Default|GetArenaLight))
  (bind _player (Variables|Default|GetPlayer))
  (bind _rootcomponent (Variables|/Script/Engine.Actor|GetRootComponent _arenalight))
  (bind _rootcomponent_2 (Variables|/Script/Engine.Actor|GetRootComponent _player))
  (bind _returnvalue (Transformation|GetWorldLocation _rootcomponent_2))
  (if (not (Variables|Default|GetArenaFightInProgress))
    _
    (else
      (Transformation|SetWorldLocation _rootcomponent (Math|Vector|MakeVector (+ (.x _returnvalue) 1e+02) (.y _returnvalue) (.z (Transformation|GetWorldLocation _rootcomponent))) false false)))
  (for _array_element (Variables|Default|GetArenaFIghtEnemies)
    (if (Variables|/Game/AlienHordeAssets/Enemies/Blueprints/BP_MonsterParent.BP_MonsterParent_C|GetIsDead _array_element)
      (Utilities|Array|RemoveItem _arenafightenemies _array_element)
      (if (Utilities|Array|IsEmpty _arenafightenemies)
        (CallFunction|AllArenaEnemiesDead)))))

(fn TriggerExplosion
  (bind _explosionspawn (Variables|Default|GetExplosionSpawn))
  (bind _explosionspawn_2 (Variables|Default|GetExplosionSpawn))
  (bind _returnvalue (Transformation|GetActorTransform _explosionspawn_2))
  (bind _returnvalue_2 (Transformation|GetActorTransform _explosionspawn))
  (bind (_location _rotation _scale) (Math|Transform|BreakTransform _returnvalue_2))
  (bind (_location_2 _rotation_2 _scale_2) (Math|Transform|BreakTransform _returnvalue))
  (bind (_roll _pitch _yaw) (Math|Rotator|BreakRotator _rotation))
  (Game|SpawnActorfromClass "/Game/StarterContent/Blueprints/Blueprint_Effect_Explosion.Blueprint_Effect_Explosion_C" (Math|Transform|MakeTransform (Math|Vector|MakeVector (.x _location_2) (.y _location_2) (- (.z _location_2) 2.5e+03)) _rotation_2 (* _scale_2 5.0)) "Undefined" "MultiplyWithRoot" 0 0)
  (for _array_element (Variables|Default|GetDoorways)
    (if (Utilities|Enum|Equal(Enum) (Utilities|GetDisplayName _array_element) "CorridorDoorway")
      (Default|Open _array_element)
      (Default|DestroyContainenment (Variables|Default|GetExplosionSpawn))
      (bind _returnvalue_3 (Game|SpawnActorfromClass "/Game/AlienHordeAssets/Enemies/Blueprints/BP_MonsterBeholder.BP_MonsterBeholder_C" (Math|Transform|MakeTransform _location (Math|Rotator|MakeRotator (+ _roll 9e+01) _pitch _yaw) (* _scale 2.0)) "AlwaysSpawn" "MultiplyWithRoot" 0 0))
      (Default|SetHealth _returnvalue_3 1e+04)
      (Default|OnSpawn _returnvalue_3)
      (Character|LaunchCharacter (Game|GetPlayerCharacter 0) "20.000000,3000.000000,0.000000" true false))))

(fn CloseCorridorDoorway
  (for _array_element (Variables|Default|GetDoorways)
    (if (Utilities|Enum|Equal(Enum) (Utilities|GetDisplayName _array_element) "CorridorDoorway")
      (Default|Close _array_element))))

(fn TriggerWeaponPickupSpotlight
  (Rendering|Components|Light|SetIntensity (Variables|/Script/Engine.Light|GetLightComponent (Variables|Default|GetFIrstWeaponSpotlight)) 1e+02))

(fn OpenFirstDoor
  (for _array_element (Variables|Default|GetDoorways)
    (if (Utilities|Enum|Equal(Enum) (Utilities|GetDisplayName _array_element) "FirstDoorway")
      (Default|Open _array_element))))