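; BP_Laser is a laser beam actor that resizes its mesh every tick.
; SetEndPoint runs a box trace, then sets the mesh's Z scale from the hit distance or LaserRange, though the trace's end offset is zero, so it covers no length.
; ChangeColor would tint a dynamic material but is never called, ChangeRotationAndLocation is empty, and right mouse prints the actor's location.
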(event EventBeginPlay
  (|CallParentFunction) ; This node is disabled and will not be called.\nDrag off pins to build functionality.
)

(event Collision|EventActorBeginOverlap
  (params (OtherActor :type Actor%20Object%20Reference))
  (|CallParentFunction OtherActor) ; This node is disabled and will not be called.\nDrag off pins to build functionality.
)

(event EventTick
  (params (DeltaSeconds :type Float%20%28single-precision%29))
  (if true
    (Variables|Default|SetLaserRange 4.0)
    (else
      (Variables|Default|SetLaserRange 1e+01)))
  (CallFunction|SetEndPoint))

(event Input|MouseEvents|RightMouseButton
  (params (Key :type Key%20Structure :default "None"))
  (:Pressed
    (Development|PrintString (Utilities|String|ToString(Vector) (Transformation|GetActorLocation)))))

(fn ConstructionScript
  (|CallParentFunction))

(fn ChangeColor
  (bind _returnvalue (Rendering|Material|CreateDynamicMaterialInstance (Variables|Default|GetSM_Parent) 0 "/Game/AlienHordeAssets/Blueprints/Laser/M_Laser.M_Laser" "None" :!class /Script/Engine.PrimitiveComponent))
  (Rendering|Material|SetVectorParameterValue _returnvalue "None" (Variables|Default|GetLaserColor) :!class /Script/Engine.MaterialInstanceDynamic))

(fn SetEndPoint
  (bind _returnvalue (Transformation|GetActorLocation))
  (bind _returnvalue_2 (Transformation|GetActorUpVector))
  (bind _returnvalue_3 (* _returnvalue_2 1.0))
  (bind _returnvalue_4 (+ _returnvalue _returnvalue_3))
  (bind _outhit (Collision|BoxTraceByChannel _returnvalue_4 (+ _returnvalue_4 (* _returnvalue_2 (* "" 1e+02))) "0.100000,0.100000,0.100000" "0, 0, 0" "TraceTypeQuery1" true 0 "None"))
  (bind _output_get (LocalVariables|SetLaserHitInfo _outhit))
  (if true
    (Variables|Default|SetLaserRange 1e+01)
    (else
      (Variables|Default|SetLaserRange 1e+01)))
  (Transformation|SetWorldScale3D (Variables|Default|GetSM_Parent) (Math|Vector|MakeVector 0.01 0.01 (Math|Float|SelectFloat (/ (+ (.Distance (Collision|BreakHitResult _output_get)) 1e+01) 1e+02) (Variables|Default|GetLaserRange) (.bBlockingHit (Collision|BreakHitResult _output_get))))))

(fn ChangeRotationandLocation)