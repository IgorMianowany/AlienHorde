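; Player character for a cursor-aimed shooter against AI enemies, handling health, death, knockback, HUD creation and camera rotation in 90-degree steps.
; Tick deprojects the mouse to rifle height to rotate body and weapon, aiming directly at hovered enemies.
; Input drives rifle, sprint and stamina components, with state checks gating shooting, laser, reload and animations.
; Roll is unfinished and DeathScript is empty, leaving ragdoll and death screen logic disconnected.
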(event Custom|Death
  ;[1 1 1] Death
  (bind _output_get (Variables|Default|SetIsDead true))
  (bind _asbp_controller (Utilities|Casting|CastToBP_Controller (Pawn|GetController)))
  (Variables|/Game/AlienHordeAssets/Blueprints/Player/BP_Controller.BP_Controller_C|SetIsPlayerDead _asbp_controller _output_get)
  (CallFunction|DeathScript))

(event Custom|ReloadFinished
  ;[1 1 1] Reload
  (Class|SkeletalMeshComponent|SetAnimClass (Variables|Character|GetMesh) "/Game/Characters/Mannequins/Animations/ABP_Manny.ABP_Manny_C"))

(event Custom|Start%20reloading
  ;[1 1 1] Reload
  (bind _can_reload (CallFunction|CanPlayerReload))
  (if _can_reload
    (Components|Animation|PlayAnimation (Variables|Character|GetMesh) "/Game/AlienHordeAssets/Animations/Reload_UE.Reload_UE" false)
    (Default|Reload (Variables|Default|GetAutomaticRIfleComponent))))

(event Custom|Stop%20Shoot%20Event
  ;[1 1 1] Shoot
  (Utilities|FlowControl|DoOnce false) ; enters at Reset
)

(event Custom|Start%20Shoot%20Event
  ;[1 1 1] Shoot
  (Utilities|FlowControl|DoOnce false
    (:Completed
      (Components|Animation|PlayAnimation (Variables|Character|GetMesh) "/Game/AlienHordeAssets/Animations/Gunplay_UE.Gunplay_UE" true))))

(event Input|EnhancedActionEvents|EnhancedInputActionIA_Sprint
  (params (ActionValue :type Boolean) (ElapsedSeconds :type Float%20%28double-precision%29) (TriggeredSeconds :type Float%20%28double-precision%29) (InputAction :type Input%20Action%20Object%20Reference :default "/Game/AlienHordeAssets/Input/Actions/IA_Sprint.IA_Sprint"))
  (bind _staminacomponent (Variables|Default|GetStaminaComponent))
  (bind _automaticriflecomponent (Variables|Default|GetAutomaticRIfleComponent))
  (bind _mesh (Variables|Character|GetMesh))
  (bind _sprintcomponent (Variables|Default|GetSprintComponent))
  (bind _charactermovement (Variables|Character|GetCharacterMovement))
  (bind _charactermovement_2 (Variables|Character|GetCharacterMovement))
  (bind _isweaponreloading (Variables|/Game/AlienHordeAssets/Blueprints/Weapons/BP_AutomaticRIfleComponent.BP_AutomaticRIfleComponent_C|GetIsWeaponReloading _automaticriflecomponent))
  (bind _stamina (Variables|/Game/AlienHordeAssets/Blueprints/Player/BP_StaminaSystem.BP_StaminaSystem_C|GetStamina _staminacomponent))
  (bind _velocity (Variables|/Script/Engine.MovementComponent|GetVelocity _charactermovement_2))
  (bind _returnvalue (Math|Vector|VectorLength _velocity))
  (bind _returnvalue_2 (<= _stamina 1.0))
  (bind _returnvalue_3 (< _returnvalue 3e+02))
  (bind _returnvalue_4 (Math|Boolean|ORBoolean _isweaponreloading _returnvalue_2 _returnvalue_3))
  ;[1 1 1] Sprint
  (:Triggered
    (if (not _returnvalue_4)
      (bind _canspend (Default|SpendStamina (Variables|Default|GetStaminaComponent) (* (Variables|/Game/AlienHordeAssets/Blueprints/Player/BP_SprintAbility.BP_SprintAbility_C|GetStaminaCost (Variables|Default|GetSprintComponent)) (Utilities|Time|GetWorldDeltaSeconds))))
      (if _canspend
        (Default|StartSprinting (Variables|Default|GetSprintComponent) (Variables|Character|GetCharacterMovement) (Variables|Character|GetMesh))
        (CallFunction|StopShootEvent))
      (else
        (Default|StopSprinting (Variables|Default|GetSprintComponent) (Variables|Character|GetCharacterMovement))
        (Variables|/Script/Engine.SkeletalMeshComponent|SetGlobalAnimRateScale _mesh 1.0 :!label _label))))
  (:Started
    (if (not _returnvalue_4)
      (Default|StartSprinting _sprintcomponent _charactermovement (Variables|Character|GetMesh))
      (Variables|/Script/Engine.SkeletalMeshComponent|SetGlobalAnimRateScale _mesh 1.67)))
  (:Completed
    (Default|StopSprinting _sprintcomponent _charactermovement)
    (goto _label)))

(event Input|EnhancedActionEvents|EnhancedInputActionIA_Roll
  (params (ActionValue :type Boolean) (ElapsedSeconds :type Float%20%28double-precision%29) (TriggeredSeconds :type Float%20%28double-precision%29) (InputAction :type Input%20Action%20Object%20Reference :default "/Game/AlienHordeAssets/Input/Actions/IA_Roll.IA_Roll"))
  ;[1 1 1] Roll unfinished
)

(event Input|EnhancedActionEvents|EnhancedInputActionIA_Shoot
  (params (ActionValue :type Boolean) (ElapsedSeconds :type Float%20%28double-precision%29) (TriggeredSeconds :type Float%20%28double-precision%29) (InputAction :type Input%20Action%20Object%20Reference :default "/Game/AlienHordeAssets/Input/Actions/IA_Shoot.IA_Shoot"))
  ;[1 1 1] Shoot
  (:Triggered
    (bind _canshoot (CallFunction|CanPlayerShoot))
    (if _canshoot
      (CallFunction|Shoot)
      (else
        (CallFunction|StopShoot)
        (if (not (Variables|/Game/AlienHordeAssets/Blueprints/Weapons/BP_AutomaticRIfleComponent.BP_AutomaticRIfleComponent_C|GetIsWeaponReloading (Variables|Default|GetAutomaticRIfleComponent)))
          (Class|SkeletalMeshComponent|SetAnimClass (Variables|Character|GetMesh) "/Game/Characters/Mannequins/Animations/ABP_Manny.ABP_Manny_C" :!label _label)))))
  (:Started
    (bind __ (CallFunction|CanPlayerAutomaticReload))
    (if __
      (CallFunction|StartReloading)))
  (:Completed
    (bind _canshoot_2 (CallFunction|CanPlayerShoot))
    (if _canshoot_2
      (CallFunction|StopShoot)
      (goto _label))))

(event Input|EnhancedActionEvents|EnhancedInputActionIA_Reload
  (params (ActionValue :type Boolean) (ElapsedSeconds :type Float%20%28double-precision%29) (TriggeredSeconds :type Float%20%28double-precision%29) (InputAction :type Input%20Action%20Object%20Reference :default "/Game/AlienHordeAssets/Input/Actions/IA_Reload.IA_Reload"))
  (bind _reloadtime (Variables|Default|GetReloadTime))
  ;[1 1 1] Set Reload Progress Bar (i dont fear god she fears me)
  (if (Variables|/Game/AlienHordeAssets/Blueprints/Weapons/BP_AutomaticRIfleComponent.BP_AutomaticRIfleComponent_C|GetIsWeaponReloading (Variables|Default|GetAutomaticRIfleComponent))
    (Variables|Default|SetTimeRemaining (- (Variables|Default|GetTimeRemaining) (Utilities|Time|GetWorldDeltaSeconds)))
    (Variables|Default|SetReloadProgress (/ (Math|Float|Clamp(Float) (- (Variables|Default|GetTimeRemaining) (Utilities|Time|GetWorldDeltaSeconds)) 0.0 _reloadtime) _reloadtime))
    (if (<= (Variables|Default|GetTimeRemaining) 0.0)
      (Utilities|FlowControl|Delay 0.5)
      (Variables|Default|SetReloadProgress 1.0)
      (Variables|Default|SetTimeRemaining 2.5))))

(event Input|EnhancedActionEvents|EnhancedInputActionIA_Reload
  (params (ActionValue :type Boolean) (ElapsedSeconds :type Float%20%28double-precision%29) (TriggeredSeconds :type Float%20%28double-precision%29) (InputAction :type Input%20Action%20Object%20Reference :default "/Game/AlienHordeAssets/Input/Actions/IA_Reload.IA_Reload"))
  ;[1 1 1] Reload
  (bind _can_reload (CallFunction|CanPlayerReload))
  (if _can_reload
    (Components|Animation|PlayAnimation (Variables|Character|GetMesh) "/Game/AlienHordeAssets/Animations/Reload_UE.Reload_UE" false)
    (Default|Reload (Variables|Default|GetAutomaticRIfleComponent))))

(event Input|EnhancedActionEvents|EnhancedInputActionIA_RotateCamera
  (params (ActionValue :type Boolean) (ElapsedSeconds :type Float%20%28double-precision%29) (TriggeredSeconds :type Float%20%28double-precision%29) (InputAction :type Input%20Action%20Object%20Reference :default "/Game/AlienHordeAssets/Input/Actions/IA_RotateCamera.IA_RotateCamera"))
  ;[1 1 1] Rotate Camera
  (:Started
    (CallFunction|RotateCamera)))

(event EventTick
  (params (DeltaSeconds :type Float%20%28single-precision%29))
  (bind _returnvalue (Game|GetPlayerController 0))
  (bind _returnvalue_2 (Game|GetPlayerCameraManager 0))
  (bind _returnvalue_3 (Game|GetPlayerController 0))
  (bind _returnvalue_4 (Game|GetPlayerCameraManager 0))
  (bind _returnvalue_5 (Transformation|GetActorRotation))
  (bind _returnvalue_6 (Game|GetPlayerController 0))
  (bind _returnvalue_7 (Transformation|GetActorLocation))
  (bind _reloadtime (Variables|Default|GetReloadTime))
  (bind _automaticrifle (Variables|Default|GetAutomaticRIfle))
  (bind _returnvalue_8 (Transformation|GetActorLocation _returnvalue_2))
  (bind _worldlocation (Game|Player|ConvertMouseLocationToWorldSpace _returnvalue_3))
  (bind _returnvalue_9 (Transformation|GetActorLocation _returnvalue_4))
  (bind _hitresult (Game|Player|GetHitResultUnderCursorbyChannel _returnvalue_6 "TraceTypeQuery3" true))
  (bind (_roll _pitch) (Math|Rotator|BreakRotator _returnvalue_5))
  (bind _hitresult_2 (Game|Player|GetHitResultUnderCursorbyChannel _returnvalue "TraceTypeQuery3" true))
  (bind _hitactor (Collision|BreakHitResult _hitresult))
  (bind _returnvalue_10 (Transformation|GetActorLocation (.hitactor _hitresult_2)))
  (bind _returnvalue_11 (- _worldlocation _returnvalue_8))
  (bind _returnvalue_12 (Math|Rotator|FindLookatRotation _returnvalue_7 _returnvalue_10))
  (bind (_roll_2 _pitch_2 _yaw) (Math|Rotator|BreakRotator _returnvalue_12))
  ;[1 1 1] Look at cursor
  (Utilities|Casting|CastToBP_AI _hitactor
    (:then
      (Variables|Default|SetEnemyUnderCursor true :!label _label))
    (:CastFailed
      (Utilities|Casting|CastToBP_CuteEnemy _hitactor
        (:then
          (goto _label))
        (:CastFailed
          (Variables|Default|SetEnemyUnderCursor false)))))
  (if (not (or (Variables|Default|GetIsDead) false))
    (bind _outhit (Collision|SphereTraceByChannel _returnvalue_9 (+ _returnvalue_9 (* (- (.WorldLocation (Game|Player|ConvertMouseLocationToWorldSpace _returnvalue_6)) _returnvalue_9) 5e+03)) 0.0 "TraceTypeQuery1" false 0 "None"))
    (Transformation|SetWorldRotation (Variables|Collision|GetCapsuleComponent) (Math|Rotator|MakeRotator _roll _pitch (+ (.yaw (Math|Rotator|FindLookatRotation (Transformation|GetActorLocation) (+ (.location _outhit) (* _returnvalue_11 (/ (- (.z (Transformation|GetWorldLocation (Variables|Default|GetAutomaticRIfle))) (.Z (Math|Vector|BreakVector (.location _outhit)))) (.Z (Math|Vector|BreakVector _returnvalue_11))))))) -9e+01)) false false)
    (if (Variables|Default|GetEnemyUnderCursor)
      (Transformation|SetWorldRotation _automaticrifle (Math|Rotator|MakeRotator (* _roll_2 1.0) (* _pitch_2 1.0) _yaw) false false)
      (else
        (Transformation|SetWorldRotation _automaticrifle (Math|Rotator|MakeRotator _roll _pitch (.yaw (Math|Rotator|FindLookatRotation (Transformation|GetActorLocation) (+ (.location _outhit) (* _returnvalue_11 (/ (- (.z (Transformation|GetWorldLocation (Variables|Default|GetAutomaticRIfle))) (.Z (Math|Vector|BreakVector (.location _outhit)))) (.Z (Math|Vector|BreakVector _returnvalue_11)))))))) false false)))
    ;[1 1 1] Set Reload Progress Bar (i dont fear god she fears me)
    (if (Variables|/Game/AlienHordeAssets/Blueprints/Weapons/BP_AutomaticRIfleComponent.BP_AutomaticRIfleComponent_C|GetIsWeaponReloading (Variables|Default|GetAutomaticRIfleComponent))
      (Variables|Default|SetTimeRemaining (- (Variables|Default|GetTimeRemaining) (Utilities|Time|GetWorldDeltaSeconds)))
      (Variables|Default|SetReloadProgress (/ (Math|Float|Clamp(Float) (- (Variables|Default|GetTimeRemaining) (Utilities|Time|GetWorldDeltaSeconds)) 0.0 _reloadtime) _reloadtime))
      (if (<= (Variables|Default|GetTimeRemaining) 0.0)
        (Utilities|FlowControl|Delay 0.5)
        (Variables|Default|SetReloadProgress 1.0)
        (Variables|Default|SetTimeRemaining 2.5)))))

(event EventBeginPlay
  (bind _automaticriflecomponent (Variables|Default|GetAutomaticRIfleComponent))
  ;[1 1 1] Add HUD to Viewport
  (bind _returnvalue (UserInterface|CreateWidget "/Game/AlienHordeAssets/ScreenWidgets/W_Player_HUD.W_Player_HUD_C" (Game|GetPlayerController 0)))
  (UserInterface|Viewport|AddtoViewport _returnvalue 0)
  (Variables|/Game/AlienHordeAssets/Blueprints/Weapons/BP_AutomaticRIfleComponent.BP_AutomaticRIfleComponent_C|SetCurrentAmmo _automaticriflecomponent (Variables|/Game/AlienHordeAssets/Blueprints/Weapons/BP_AutomaticRIfleComponent.BP_AutomaticRIfleComponent_C|GetMaxAmmo _automaticriflecomponent)))

(fn ConstructionScript)

(fn DeathScript)

(fn TakeDamage
  (params (Damage :type Float%20%28double-precision%29))
  (bind _output_get (Variables|Default|SetHealth (- (Variables|Default|GetHealth) Damage)))
  (if (not (> _output_get 0.0))
    (CallFunction|Death)))

(fn KnockBack
  (params (Location :type Vector))
  (Character|LaunchCharacter Location true true))

(fn RecoilWeapon
  (bind _automaticrifle (Variables|Default|GetAutomaticRIfle))
  (Transformation|SetRelativeLocation _automaticrifle (- (.location (Transformation|GetRelativeTransform _automaticrifle)) (Variables|Default|GetWeaponRecoilDistance)) false false))

(fn RecoilWeaponBack
  (bind _automaticrifle (Variables|Default|GetAutomaticRIfle))
  (Transformation|SetRelativeLocation _automaticrifle (+ (.location (Transformation|GetRelativeTransform _automaticrifle)) (Variables|Default|GetWeaponRecoilDistance)) false false))

(fn ResetGunPosition
  (Transformation|SetRelativeLocation (Variables|Default|GetAutomaticRIfle) "0.000000,30.000000,37.000000" false false))

(fn SpawnLaser)

(fn Shoot
  (bind _laser (CallFunction|GetLaser))
  (Variables|/Game/AlienHordeAssets/Blueprints/Laser/BP_Laser.BP_Laser_C|SetIsPlayerShooting _laser true)
  (Variables|/Game/AlienHordeAssets/Blueprints/Weapons/BP_AutomaticRIfleComponent.BP_AutomaticRIfleComponent_C|SetBulletSpawnTransform (Variables|Default|GetAutomaticRIfleComponent) (Transformation|GetWorldTransform (Variables|Default|GetBulletSpawn)))
  (Default|StartShooting (Variables|Default|GetAutomaticRIfleComponent) (Variables|Default|GetAutomaticRIfle))
  (CallFunction|StartShootEvent))

(fn StopShoot
  (bind _laser (CallFunction|GetLaser))
  (Variables|/Game/AlienHordeAssets/Blueprints/Laser/BP_Laser.BP_Laser_C|SetIsPlayerShooting _laser false)
  (Default|StopShooting (Variables|Default|GetAutomaticRIfleComponent))
  (CallFunction|StopShootEvent))

(fn CanPlayerShoot
  (bind _automaticriflecomponent (Variables|Default|GetAutomaticRIfleComponent))
  (return (not (Math|Boolean|ORBoolean (Variables|Default|GetIsDead) (Variables|/Game/AlienHordeAssets/Blueprints/Weapons/BP_AutomaticRIfleComponent.BP_AutomaticRIfleComponent_C|GetIsWeaponReloading _automaticriflecomponent) (<= (Variables|/Game/AlienHordeAssets/Blueprints/Weapons/BP_AutomaticRIfleComponent.BP_AutomaticRIfleComponent_C|GetCurrentAmmo _automaticriflecomponent) 0) (Variables|/Game/AlienHordeAssets/Blueprints/Player/BP_SprintAbility.BP_SprintAbility_C|GetIsSprinting (Variables|Default|GetSprintComponent)) (Variables|Default|GetIsRolling)))))

(fn CanPlayerAutomaticReload
  (bind _automaticriflecomponent (Variables|Default|GetAutomaticRIfleComponent))
  (return (Math|Boolean|ANDBoolean (not (Variables|Default|GetIsDead)) (not (Variables|/Game/AlienHordeAssets/Blueprints/Weapons/BP_AutomaticRIfleComponent.BP_AutomaticRIfleComponent_C|GetIsWeaponReloading _automaticriflecomponent)) (== (Variables|/Game/AlienHordeAssets/Blueprints/Weapons/BP_AutomaticRIfleComponent.BP_AutomaticRIfleComponent_C|GetCurrentAmmo _automaticriflecomponent) 0) (not (Variables|Default|GetIsRolling)) (not (Variables|/Game/AlienHordeAssets/Blueprints/Player/BP_SprintAbility.BP_SprintAbility_C|GetIsSprinting (Variables|Default|GetSprintComponent))))))

(fn CanPlayerReload
  (bind _automaticriflecomponent (Variables|Default|GetAutomaticRIfleComponent))
  (return (Math|Boolean|ANDBoolean (not (Variables|Default|GetIsDead)) (not (Variables|/Game/AlienHordeAssets/Blueprints/Weapons/BP_AutomaticRIfleComponent.BP_AutomaticRIfleComponent_C|GetIsWeaponReloading _automaticriflecomponent)) (< (Variables|/Game/AlienHordeAssets/Blueprints/Weapons/BP_AutomaticRIfleComponent.BP_AutomaticRIfleComponent_C|GetCurrentAmmo _automaticriflecomponent) (Variables|/Game/AlienHordeAssets/Blueprints/Weapons/BP_AutomaticRIfleComponent.BP_AutomaticRIfleComponent_C|GetMaxAmmo _automaticriflecomponent)) (> (Variables|/Game/AlienHordeAssets/Blueprints/Weapons/BP_AutomaticRIfleComponent.BP_AutomaticRIfleComponent_C|GetMagazines _automaticriflecomponent) 0) (not (Variables|/Game/AlienHordeAssets/Blueprints/Player/BP_SprintAbility.BP_SprintAbility_C|GetIsSprinting (Variables|Default|GetSprintComponent))))))

(fn GetLaser
  (bind _asbp_laser_spawn (Utilities|Casting|CastToBP_LaserSpawn (Variables|/Script/Engine.ChildActorComponent|GetChildActor (Variables|Default|GetLaserSpawn))))
  (return (Variables|/Game/AlienHordeAssets/Blueprints/Laser/BP_LaserSpawn.BP_LaserSpawn_C|GetChildLaser _asbp_laser_spawn)))

(fn RotateCamera
  (bind _springarm (Variables|Camera|GetSpringArm))
  (bind _returnvalue (Class|SpringArmComponent|GetTargetRotation _springarm))
  (Transformation|SetWorldRotation _springarm (Math|Rotator|MakeRotator (.roll _returnvalue) (.pitch _returnvalue) (+ (.yaw _returnvalue) 9e+01)) false false))