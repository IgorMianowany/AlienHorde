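; BP_Bullet is a projectile actor that damages enemies on contact, with its damage amount set at BeginPlay.
; An overlap on its CollisionHitbox counts as a hit if the other component is tagged Aim or lacks the Passable tag.
; A hit casts the other actor to BP_AI, then BP_CuteEnemy, calls TakeDamage on a match, and destroys the bullet either way.
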(event OnComponentBeginOverlap(CollisionHitbox)
  (params (OverlappedComponent :type Primitive%20Component%20Object%20Reference) (OtherActor :type Actor%20Object%20Reference) (OtherComp :type Primitive%20Component%20Object%20Reference) (OtherBodyIndex :type Integer) (bFromSweep :type Boolean) (SweepResult :type Hit%20Result%20Structure%20%28by%20ref%29))
  (bind _damage (Variables|Default|GetDamage))
  (if (Components|ComponentHasTag OtherComp "Aim")
    (bind _asbp_ai (Utilities|Casting|CastToBP_AI OtherActor :!label _label)
      (:then
        (Default|TakeDamage _asbp_ai _damage))
      (:CastFailed
        (bind _asbp_cute_enemy (Utilities|Casting|CastToBP_CuteEnemy OtherActor)
          (:then
            (Default|TakeDamage _asbp_cute_enemy _damage))
          (:CastFailed
            _))))
    (Actor|DestroyActor)
    (elif (not (Components|ComponentHasTag OtherComp "Passable"))
      (goto _label))))

(event EventBeginPlay
  (Variables|Default|SetDamage 5e+01))

(fn ConstructionScript)