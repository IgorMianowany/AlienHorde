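; Game mode for the alien horde game that sets up and triggers enemy spawning.
; On BeginPlay it spawns a single BP_EnemySpawn at a hardcoded location and stores it as the SpawnPoints array.
; The TriggerEnemySpawn event calls a function that spawns one BP_AI at each point's transform and calls its OnSpawn.
; A 100-iteration batch loop and an offset transform are left unconnected.
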(event Custom|Event%20TriggerEnemySpawn
  (CallFunction|TriggerEnemySpawn))

(event EventBeginPlay
  (bind _returnvalue (Game|SpawnActorfromClass "/Game/AlienHordeAssets/Blueprints/Enemy/BP_EnemySpawn.BP_EnemySpawn_C" (Math|Transform|MakeTransform "2270.000000,1683.000000,25.000000") "Undefined" "MultiplyWithRoot" 0 0))
  (Variables|Default|SetSpawnPoints (Utilities|Array|MakeArray _returnvalue)))

(fn ConstructionScript)

(fn TriggerEnemySpawn
  (for _array_element (Variables|Default|GetSpawnPoints)
    (bind _returnvalue (Game|SpawnActorfromClass "/Game/AlienHordeAssets/Blueprints/Enemy/BP_AI.BP_AI_C" (Transformation|GetActorTransform _array_element) "Undefined" "MultiplyWithRoot" 0 0))
    (Default|OnSpawn _returnvalue)))