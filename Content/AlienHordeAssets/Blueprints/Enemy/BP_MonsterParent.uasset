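; Parent enemy character that patrols, chases the player and attacks in melee.
; A Timeline drives AI moves between points either side of its start until pawn sensing, spawning or damage switches it to chasing.
; Attack hitbox overlap starts a looping timer that damages and knocks back the player while in range.
; TakeDamage updates the health text and, at zero, flags death and disables collision.
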(event OnComponentBeginOverlap(Hitbox)
  (params (OverlappedComponent :type Primitive%20Component%20Object%20Reference) (OtherActor :type Actor%20Object%20Reference) (OtherComp :type Primitive%20Component%20Object%20Reference) (OtherBodyIndex :type Integer) (bFromSweep :type Boolean) (SweepResult :type Hit%20Result%20Structure%20%28by%20ref%29))
  (bind _asbp_player_character (Utilities|Casting|CastToBP_PlayerCharacter OtherActor)))

(event OnComponentBeginOverlap(AttackHitbox)
  (params (OverlappedComponent :type Primitive%20Component%20Object%20Reference) (OtherActor :type Actor%20Object%20Reference) (OtherComp :type Primitive%20Component%20Object%20Reference) (OtherBodyIndex :type Integer) (bFromSweep :type Boolean) (SweepResult :type Hit%20Result%20Structure%20%28by%20ref%29))
  ;[1 1 1] Run at Player Events
  (Variables|Default|SetIsPlayerInRange true)
  (Utilities|Time|SetTimerbyEvent (delegate Custom|Attack%20Cooldown) (Variables|Default|GetAttackSpeed) true true)
  (CallFunction|Attack OtherActor OtherComp)
  (Utilities|FlowControl|Delay 0.5)
  (if (Variables|Default|GetIsAttacking)
    (Variables|Default|SetIsAttacking false)))

(event OnSeePawn(PawnSensing)
  (params (Pawn :type Pawn%20Object%20Reference))
  ;[1 1 1] Run at Player Events
  (CallFunction|RunatPlayer (Game|Player|GetPlayerPawn 0)))

(event OnComponentEndOverlap(AttackHitbox)
  (params (OverlappedComponent :type Primitive%20Component%20Object%20Reference) (OtherActor :type Actor%20Object%20Reference) (OtherComp :type Primitive%20Component%20Object%20Reference) (OtherBodyIndex :type Integer))
  ;[1 1 1] Run at Player Events
  (Utilities|Casting|CastToBP_PlayerCharacter OtherActor)
  (Variables|Default|SetIsPlayerInRange false))

(event Custom|Event%20Take%20Damage
  ;[1 1 1] Run at Player Events
  (CallFunction|RunatPlayer (Game|Player|GetPlayerPawn 0)))

(event Custom|On%20Spawn
  ;[1 1 1] Run at Player Events
  (CallFunction|RunatPlayer (Game|Player|GetPlayerPawn 0)))

(event Custom|Event%20AfterTakeDamage
  ;[1 1 1] Run at Player Events
  (Utilities|FlowControl|Delay 0.3)
  (Variables|Default|SetIsHit false))

(event Custom|Attack%20Cooldown
  ;[1 1 1] Run at Player Events
  (CallFunction|Attack (stale OnComponentBeginOverlap(AttackHitbox) OtherActor) (stale OnComponentBeginOverlap(AttackHitbox) OtherComp))
  (Utilities|FlowControl|Delay 0.5)
  (if (Variables|Default|GetIsAttacking)
    (Variables|Default|SetIsAttacking false)))

(event Collision|EventActorBeginOverlap
  (params (OtherActor :type Actor%20Object%20Reference))
  (Utilities|Casting|CastToBP_Bullet OtherActor))

(event EventTick
  (params (DeltaSeconds :type Float%20%28single-precision%29))
  ;[1 1 1] Patrol movement
  (if (Variables|Default|GetCanSeePlayer)
    (Utilities|FlowControl|DoOnce false
      (:Completed
        (bind _patrol_track (Timeline|Timeline Stop)
          (:Update
            (AI|Navigation|MovetoLocation (AI|GetAIController self) (Math|Vector|Lerp(Vector) (stale EventBeginPlay _output_get_2) (stale EventBeginPlay _output_get_3) _patrol_track) -1.0 true true false true 0)))))))

(event EventBeginPlay
  (bind _returnvalue (Transformation|GetActorLocation))
  ;[1 1 1] Patrol movement
  (bind _output_get (Variables|Default|SetHealth%20Points 1e+02))
  (Rendering|Components|TextRender|SetText (Variables|Default|GetHealth%20Display) (Utilities|Text|ToText(Float) _output_get "HalfToEven"))
  (bind _output_get_2 (Variables|Default|SetStart (+ _returnvalue "-500.000000,0.000000,0.000000")))
  (bind _output_get_3 (Variables|Default|SetEnd (+ _returnvalue "500.000000,0.000000,0.000000")))
  (bind _patrol_track (Timeline|Timeline PlayFromStart)
    (:Update
      (AI|Navigation|MovetoLocation (AI|GetAIController self) (Math|Vector|Lerp(Vector) _output_get_2 _output_get_3 _patrol_track) -1.0 true true false true 0))))

(fn ConstructionScript)

(fn TakeDamage
  (params (Damage :type Float%20%28double-precision%29))
  (if (> (Variables|Default|GetHealth%20Points) 0.0)
    (Variables|Default|SetIsHit true)
    (bind _output_get (Variables|Default|SetHealth%20Points (- (Variables|Default|GetHealth%20Points) Damage)))
    (Rendering|Components|TextRender|SetText (Variables|Default|GetHealth%20Display) (Utilities|Text|ToText(Float) (Variables|Default|GetHealth%20Points) "HalfToEven"))
    (CallFunction|EventTakeDamage)
    (CallFunction|EventAfterTakeDamage)
    (if (<= _output_get 0.0)
      (Utilities|FlowControl|DoOnce false
        (:Completed
          (Variables|Default|SetIsDead true)
          (Collision|SetActorEnableCollision false))))))

(fn RunatPlayer
  (params (Player :type Pawn%20Object%20Reference))
  (bind _asbp_player_character (Utilities|Casting|CastToBP_PlayerCharacter Player))
  (Variables|Default|SetCanSeePlayer true)
  (if (not (Variables|Default|GetIsDead))
    (AI|Navigation|MovetoActor (AI|GetAIController self) _asbp_player_character -1.0 false true true "/Script/NavigationSystem.NavigationQueryFilter")
    (else
      (Pawn|Components|CharacterMovement|DisableMovement (Variables|Character|GetCharacterMovement))
      (Collision|SetCollisionEnabled (Variables|Collision|GetCapsuleComponent) "NoCollision"))))

(fn Attack
  (params (Player%20Actor :type Actor%20Object%20Reference) (Component :type Primitive%20Component%20Object%20Reference))
  (if (and (Variables|Default|GetIsPlayerInRange) (not (Variables|Default|GetIsDead)))
    (bind _asbp_player_character (Utilities|Casting|CastToBP_PlayerCharacter Player%20Actor))
    (Variables|Default|SetIsAttacking true)
    (Default|TakeDamage _asbp_player_character (Variables|Default|GetAttackDamage))
    (Default|KnockBack _asbp_player_character (* (Math|Vector|GetForwardVector (Transformation|GetWorldRotation (Variables|Collision|GetCapsuleComponent))) 1e+03))))