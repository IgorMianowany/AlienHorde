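; BP_Enemy is a patrolling enemy that kills the player on hitbox contact and shows its health as text.
; A looping-style Patrol timeline lerps it between two points either side of its spawn location along world X.
; Tick pauses the timeline while the player overlaps PlayerDetection and resumes it otherwise.
; TakeDamage lowers health and destroys the actor at zero; the bullet overlap event only casts, with no effect.
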(event OnComponentBeginOverlap(Hitbox)
  (params (OverlappedComponent :type Primitive%20Component%20Object%20Reference) (OtherActor :type Actor%20Object%20Reference) (OtherComp :type Primitive%20Component%20Object%20Reference) (OtherBodyIndex :type Integer) (bFromSweep :type Boolean) (SweepResult :type Hit%20Result%20Structure%20%28by%20ref%29))
  (bind _asbp_player_character (Utilities|Casting|CastToBP_PlayerCharacter OtherActor))
  (Default|Death _asbp_player_character))

(event OnComponentBeginOverlap(PlayerDetection)
  (params (OverlappedComponent :type Primitive%20Component%20Object%20Reference) (OtherActor :type Actor%20Object%20Reference) (OtherComp :type Primitive%20Component%20Object%20Reference) (OtherBodyIndex :type Integer) (bFromSweep :type Boolean) (SweepResult :type Hit%20Result%20Structure%20%28by%20ref%29))
  ;[1 1 1] Detect Player
  (Utilities|Casting|CastToBP_PlayerCharacter OtherActor)
  (Variables|Default|SetIsPlayerNearby true))

(event OnComponentEndOverlap(PlayerDetection)
  (params (OverlappedComponent :type Primitive%20Component%20Object%20Reference) (OtherActor :type Actor%20Object%20Reference) (OtherComp :type Primitive%20Component%20Object%20Reference) (OtherBodyIndex :type Integer))
  ;[1 1 1] Detect Player
  (Utilities|Casting|CastToBP_PlayerCharacter OtherActor)
  (Variables|Default|SetIsPlayerNearby false))

(event EventBeginPlay
  (bind _returnvalue (Transformation|GetActorLocation))
  ;[1 1 1] Patrol movement
  (bind _output_get (Variables|Default|SetHealth%20Points 1e+02))
  (Rendering|Components|TextRender|SetText (Variables|Default|GetHealth%20Display) (Utilities|Text|ToText(Float) _output_get "HalfToEven"))
  (bind _output_get_2 (Variables|Default|SetStart (+ _returnvalue "-300.000000,0.000000,0.000000")))
  (bind _output_get_3 (Variables|Default|SetEnd (+ _returnvalue "300.000000,0.000000,0.000000")))
  (bind _patrol_track (Timeline|Patrol PlayFromStart)
    (:Update
      (Transformation|SetActorLocation (Math|Vector|Lerp(Vector) _output_get_2 _output_get_3 _patrol_track) false false))))

(event Collision|EventActorBeginOverlap
  (params (OtherActor :type Actor%20Object%20Reference))
  (Utilities|Casting|CastToBP_Bullet OtherActor))

(event EventTick
  (params (DeltaSeconds :type Float%20%28single-precision%29))
  ;[1 1 1] Patrol movement
  (if (Variables|Default|GetIsPlayerNearby)
    (bind _patrol_track (Timeline|Patrol Stop)
      (:Update
        (Transformation|SetActorLocation (Math|Vector|Lerp(Vector) (stale EventBeginPlay _output_get_2) (stale EventBeginPlay _output_get_3) _patrol_track) false false)))
    (else
      (Timeline|Patrol Play))))

(fn ConstructionScript)

(fn TakeDamage
  (params (Damage :type Float%20%28double-precision%29))
  (bind _output_get (Variables|Default|SetHealth%20Points (- (Variables|Default|GetHealth%20Points) Damage)))
  (Rendering|Components|TextRender|SetText (Variables|Default|GetHealth%20Display) (Utilities|Text|ToText(Float) (Variables|Default|GetHealth%20Points) "HalfToEven"))
  (if (not (> _output_get 0.0))
    (Variables|Default|SetIsDead true)
    (Actor|DestroyActor)))