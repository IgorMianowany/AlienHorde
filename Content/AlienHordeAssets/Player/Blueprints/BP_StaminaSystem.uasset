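; Stamina system for the player that tracks a stamina pool, starting full, and regenerates it over time.
; A looping TickStamina timer, rather than event Tick, adds regen and clamps it to the maximum.
; SpendStamina deducts only when enough is available, reports success, and calls PauseStaminaTick to halt regen.
; A named timer resumes regen after the delay, so each new timed pause restarts the countdown.
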(event EventBeginPlay
  (Variables|Default|SetStamina (Variables|Default|GetMaxStamina))
  (bind _returnvalue (Utilities|Time|SetTimerbyFunctionName 0 "TickStamina" (Variables|Default|GetStaminaTickRate) true))
  (Variables|Default|SetStaminaTickTimer _returnvalue))

(event EventTick
  (params (DeltaSeconds :type Float%20%28single-precision%29)))

(fn TickStamina
  (Variables|Default|SetStamina (Math|Float|Clamp(Float) (+ (Variables|Default|GetStamina) (* (Variables|Default|GetStaminaRegenRate) (Variables|Default|GetStaminaTickRate))) 0.0 (Variables|Default|GetMaxStamina))))

(fn StartStaminaTick
  (Utilities|Time|UnpauseTimerbyHandle (Variables|Default|GetStaminaTickTimer)))

(fn StopStaminaTick
  (Utilities|Time|PauseTimerbyHandle (Variables|Default|GetStaminaTickTimer)))

(fn SpendStamina
  (params (Amount :type Float%20%28double-precision%29))
  (if (and (> Amount 0.0) (>= (Variables|Default|GetStamina) Amount))
    (Variables|Default|SetStamina (Math|Float|Clamp(Float) (- (Variables|Default|GetStamina) Amount) 0.0 (Variables|Default|GetMaxStamina)))
    (CallFunction|PauseStaminaTick (Variables|Default|GetStaminaSpentPauseDuration))
    (return true)
    (else
      (return false))))

(fn PauseStaminaTick
  (params (Duration :type Float%20%28double-precision%29))
  (Utilities|Time|PauseTimerbyHandle (Variables|Default|GetStaminaTickTimer))
  (if (> Duration 0.0)
    (Utilities|Time|SetTimerbyFunctionName 0 "StartStaminaTick" Duration)))