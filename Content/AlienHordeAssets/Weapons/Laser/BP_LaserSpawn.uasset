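; BP_LaserSpawn is a laser emitter actor that creates and carries a BP_Laser beam.
; On BeginPlay it records its display name as an Id, then spawns a scaled-down BP_Laser at its Arrow, passing range, color and a reference to itself.
; Every Tick it copies its own location and rotation onto the spawned laser's root, so the beam follows the actor's origin without attachment.
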(event EventBeginPlay
  (bind _self self)
  (|CallParentFunction)
  (Variables|Default|SetSpawnReference _self)
  (Variables|Default|SetId (Utilities|GetDisplayName _self))
  (bind _returnvalue (Game|SpawnActorfromClass "/Game/AlienHordeAssets/Weapons/Laser/BP_Laser.BP_Laser_C" (Math|Transform|MakeTransform (Transformation|GetWorldLocation (Variables|Default|GetArrow)) (Transformation|GetActorRotation) "0.100000,0.100000,0.100000") "Undefined" "MultiplyWithRoot" 0 1e+01 (Variables|Default|GetLaserColor) (Variables|Default|GetSpawnReference) 0))
  (Variables|Default|SetChildLaser _returnvalue))

(event EventTick
  (params (DeltaSeconds :type Float%20%28single-precision%29))
  (bind _childlaser (Variables|Default|GetChildLaser))
  (bind _rootcomponent (Variables|/Script/Engine.Actor|GetRootComponent _childlaser))
  (Transformation|SetWorldRotation _rootcomponent (Transformation|GetActorRotation) false false)
  (Transformation|SetWorldLocation _rootcomponent (Transformation|GetActorLocation) false false))

(fn ConstructionScript
  (|CallParentFunction))