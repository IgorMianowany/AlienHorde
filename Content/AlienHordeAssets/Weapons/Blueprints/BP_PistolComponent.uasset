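; Pistol weapon component that handles firing, ammo and magazine-based reloading.
; Tick counts down a fire-rate timer, which gates StartShooting along with ammo to spawn BP_Bullet, an attached Niagara muzzle flash and a gunshot sound.
; Reload runs on a timer, then refills ammo, spends a magazine and notifies BP_PlayerCharacter.
; StopShooting clears a timer handle that only disconnected auto-fire code sets, so each StartShooting call fires at most one shot.
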(event EventBeginPlay)

(event EventTick
  (params (DeltaSeconds :type Float%20%28single-precision%29))
  (Variables|Default|SetFirerateTimer (- (Variables|Default|GetFirerateTimer) DeltaSeconds)))

(fn StartShooting
  (params (AttachableComponent :type Scene%20Component%20Object%20Reference))
  (bind _canshoot (CallFunction|CanWeaponShoot))
  (if _canshoot
    (Variables|Default|SetFirerateTimer (Variables|Default|GetFirerate))
    (Variables|Default|SetCurrentAmmo (- (Variables|Default|GetCurrentAmmo) 1))
    (Game|SpawnActorfromClass "/Game/AlienHordeAssets/Weapons/Blueprints/BP_Bullet.BP_Bullet_C" (Variables|Default|GetBulletSpawnTransform) "AdjustIfPossibleButAlwaysSpawn" "MultiplyWithRoot" 0 (Variables|Default|GetBulletDamage) 0)
    (bind _returnvalue (Niagara|SpawnSystemAttached "/Game/AlienHordeAssets/Weapons/VFX/NS_Gunfire.NS_Gunfire" AttachableComponent "BulletSpawn" "0, 0, 0" "0.000000,90.000000,0.000000" "KeepRelativeOffset" true))
    (Transformation|AttachComponentToComponent _returnvalue AttachableComponent "BulletSpawn" "KeepWorld" "KeepWorld" "SnapToTarget" true)
    (Audio|PlaySoundatLocation "/Game/FPWeapon/Audio/FirstPersonTemplateWeaponFire02.FirstPersonTemplateWeaponFire02" (.location (Variables|Default|GetBulletSpawnTransform)) "0, 0, 0" 1.0 1.0 0.0 0 0 0 0)))

(fn StopShooting
  (Utilities|Time|ClearandInvalidateTimerbyHandle (Variables|Default|GetShootTimerHandle)))

(fn CanWeaponShoot
  (return (and (<= (Variables|Default|GetFirerateTimer) 0.0) (> (Variables|Default|GetCurrentAmmo) 0))))

(fn Reload
  (Utilities|Time|SetTimerbyFunctionName 0 "Reload Logic" (Variables|Default|GetReloadTime))
  (Variables|Default|SetIsWeaponReloading true))

(fn ReloadLogic
  (Variables|Default|SetCurrentAmmo (Variables|Default|GetMaxAmmo))
  (Variables|Default|SetMagazines (- (Variables|Default|GetMagazines) 1))
  (Variables|Default|SetIsWeaponReloading false)
  (bind _asbp_player_character (Utilities|Casting|CastToBP_PlayerCharacter (Game|GetPlayerCharacter 0)))
  (Default|ReloadFinished _asbp_player_character))

(fn RefillMagazines
  (Variables|Default|SetMagazines (Variables|Default|GetMaxMagazines)))