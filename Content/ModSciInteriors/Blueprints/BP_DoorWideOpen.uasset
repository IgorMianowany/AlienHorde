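; BP_DoorWideOpen is a key-locked door that swings open when a player character holding a key enters its Trigger.
; The overlap plays a timeline that feeds OperateDoor, which rotates StaticMesh by lerping between the DoorClosed and DoorOpen vectors as Euler angles.
; Any actor leaving the trigger reverses the timeline, without a key or class check.
; Disconnected leftover nodes hold unused sliding and steam-effect logic.
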(event OnComponentBeginOverlap(Trigger)
  (params (OverlappedComponent :type Primitive%20Component%20Object%20Reference) (OtherActor :type Actor%20Object%20Reference) (OtherComp :type Primitive%20Component%20Object%20Reference) (OtherBodyIndex :type Integer) (bFromSweep :type Boolean) (SweepResult :type Hit%20Result%20Structure%20%28by%20ref%29))
  (bind _asbp_player_character (Utilities|Casting|CastToBP_PlayerCharacter OtherActor))
  (if (Variables|/Game/AlienHordeAssets/Player/Blueprints/BP_PlayerCharacter.BP_PlayerCharacter_C|GetHasKey _asbp_player_character)
    (bind _doorposition (Timeline|Timeline_0 Play)
      (:Update
        (CallFunction|OperateDoor _doorposition)))))

(event OnComponentEndOverlap(Trigger)
  (params (OverlappedComponent :type Primitive%20Component%20Object%20Reference) (OtherActor :type Actor%20Object%20Reference) (OtherComp :type Primitive%20Component%20Object%20Reference) (OtherBodyIndex :type Integer))
  (bind _doorposition (Timeline|Timeline_0 Reverse)
    (:Update
      (CallFunction|OperateDoor _doorposition))))

(fn ConstructionScript)

(fn OperateDoor
  (params (Position :type Float%20%28double-precision%29))
  (bind _dooropen (Variables|Door|GetDoorOpen))
  (bind _doorclosed (Variables|Door|GetDoorClosed))
  (bind _returnvalue (Math|Vector|Lerp(Vector) _doorclosed _dooropen Position))
  (Transformation|SetRelativeRotation (Variables|Default|GetStaticMesh) (Math|Rotator|MakeRotator (.x _returnvalue) (.y _returnvalue) (.z _returnvalue)) false false))